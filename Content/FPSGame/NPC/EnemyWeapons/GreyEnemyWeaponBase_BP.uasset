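; Base enemy weapon Blueprint that fires hitscan rounds on request, gated by a DoOnce.
; Each round activates the projectile particle system, plays a sound and line-traces forward from the muzzle on the Camera channel.
; A hit applies point damage, reports it to AI damage sensing and, after a short delay, deactivates the particles.
; A cyclic-rate timer broadcasts OnWeaponFired and resets the gate.
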(event Custom|OnFireRequested
  (Utilities|FlowControl|DoOnce false
    (:Completed
      (CallFunction|FireRound)
      (Utilities|Time|SetTimerbyFunctionName 0 "Ready" (Variables|Default|GetCyclicRate)))))

(event Custom|FireRound
  (bind _returnvalue (Components|GetOwner))
  (bind _muzzleposition (Variables|Default|GetMuzzlePosition))
  (bind _returnvalue_2 (Game|GetInstigatorController _returnvalue))
  (bind _returnvalue_3 (Transformation|GetWorldLocation _muzzleposition))
  (Components|Activation|SetActive (Variables|Default|GetProectile_System) true true)
  (Audio|PlaySoundatLocation "/Game/FPSGame/NPC/Audio/EnemyWeaponFire.EnemyWeaponFire" _returnvalue_3 "0, 0, 0" 1.0 1.0 0.0 0 0 0)
  (bind (_outhit _returnvalue_4) (Collision|LineTraceByChannel _returnvalue_3 (+ _returnvalue_3 (* (Math|Vector|GetForwardVector (Variables|Default|GetMuzzlePosition)) (Variables|Default|GetWeaponRange))) "TraceTypeQuery2" false 0 "None" true "(R=1.000000,G=0.000000,B=0.000000,A=1.000000)" "(R=0.000000,G=1.000000,B=0.000000,A=1.000000)" 2.0))
  (if _returnvalue_4
    (Game|Damage|ApplyPointDamage (.HitActor (Collision|BreakHitResult _outhit)) (Variables|Default|GetWeaponDamage) (.ImpactNormal (Collision|BreakHitResult _outhit)) _outhit _returnvalue_2 self "/Script/Engine.DamageType")
    (Class|AISenseDamage|ReportDamageEvent (.HitActor (Collision|BreakHitResult _outhit)) _returnvalue_2 (Variables|Default|GetWeaponDamage) (.Location (Collision|BreakHitResult _outhit)) "0, 0, 0" "None")
    (Utilities|FlowControl|Delay 0.2)
    (Components|Activation|Deactivate (Variables|Default|GetProectile_System))))

(event Custom|Ready
  (Default|CallOnWeaponFired)
  (Utilities|FlowControl|DoOnce false) ; enters at Reset
)

(fn ConstructionScript)