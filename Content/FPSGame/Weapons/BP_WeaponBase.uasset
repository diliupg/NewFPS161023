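; Base weapon for the FPS player, handling firing, ammo, reloading and recoil.
; StartShooting spends a round, auto-reloads on empty and runs hitscan camera traces, repeated per shotgun pellet with random spread unless aiming.
; Shots message damage to the hit actor, spawn impact effects and play a reversing recoil Timeline on controller input.
; Helper functions handle type-matched pickups, magazine refills and shell-by-shell shotgun loading, while the player's aim events toggle aiming.
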(event Custom|AutoReloadOnEmpty
  (bind _weapontype (Variables|WeaponData|GetWeaponType))
  ;[0 0.3437 1 1 12] Automatically calls reload event
  (if (or (Utilities|Enum|Equal(Enum) _weapontype "NewEnumerator3") (Utilities|Enum|Equal(Enum) _weapontype "NewEnumerator2"))
    (Utilities|FlowControl|Delay 0.4) ; Wait for the sniper shot to complete
    (Default|Reload (Variables|Default|GetPlayer))
    (CallFunction|WeaponAimExit)
    (else
      (Default|Reload (Variables|Default|GetPlayer)))))

(event Custom|StartRecoil
  (bind _returnvalue (Game|GetPlayerCharacter 0))
  ;[0 0.5547 1 1 12] Adds recoil effect to weapons
  (bind (_direction _alpha) (Timeline|Recoil PlayFromStart)
    (:Update
      (switch Utilities|FlowControl|Switch|SwitchonETimelineDirection _direction
        (:Forward
          (Pawn|Input|AddControllerPitchInput _returnvalue (Math|Float|Lerp 0.0 (Variables|WeaponData|GetWeaponKick) _alpha))
          (Pawn|Input|AddControllerYawInput (Game|GetPlayerCharacter 0) (Math|Random|RandomFloatinRange -0.15 0.15)))
        (:Backward
          (Pawn|Input|AddControllerPitchInput _returnvalue (* (Math|Float|Lerp 0.0 (Variables|WeaponData|GetWeaponKick) _alpha) -1.0)))))
    (:Finished
      (CallFunction|ReverseRecoil)
      (Utilities|FlowControl|RetriggerableDelay 0.05)
      (CallFunction|StopRecoil))))

(event Custom|StopRecoil
  (bind _returnvalue (Game|GetPlayerCharacter 0))
  ;[0 0.5547 1 1 12] Adds recoil effect to weapons
  (bind (_direction _alpha) (Timeline|Recoil Stop)
    (:Update
      (switch Utilities|FlowControl|Switch|SwitchonETimelineDirection _direction
        (:Forward
          (Pawn|Input|AddControllerPitchInput _returnvalue (Math|Float|Lerp 0.0 (Variables|WeaponData|GetWeaponKick) _alpha))
          (Pawn|Input|AddControllerYawInput (Game|GetPlayerCharacter 0) (Math|Random|RandomFloatinRange -0.15 0.15)))
        (:Backward
          (Pawn|Input|AddControllerPitchInput _returnvalue (* (Math|Float|Lerp 0.0 (Variables|WeaponData|GetWeaponKick) _alpha) -1.0)))))
    (:Finished
      (CallFunction|ReverseRecoil)
      (Utilities|FlowControl|RetriggerableDelay 0.05)
      (CallFunction|StopRecoil))))

(event Custom|ReverseRecoil
  (bind _returnvalue (Game|GetPlayerCharacter 0))
  ;[0 0.5547 1 1 12] Adds recoil effect to weapons
  (bind (_direction _alpha) (Timeline|Recoil Reverse)
    (:Update
      (switch Utilities|FlowControl|Switch|SwitchonETimelineDirection _direction
        (:Forward
          (Pawn|Input|AddControllerPitchInput _returnvalue (Math|Float|Lerp 0.0 (Variables|WeaponData|GetWeaponKick) _alpha))
          (Pawn|Input|AddControllerYawInput (Game|GetPlayerCharacter 0) (Math|Random|RandomFloatinRange -0.15 0.15)))
        (:Backward
          (Pawn|Input|AddControllerPitchInput _returnvalue (* (Math|Float|Lerp 0.0 (Variables|WeaponData|GetWeaponKick) _alpha) -1.0)))))
    (:Finished
      (CallFunction|ReverseRecoil)
      (Utilities|FlowControl|RetriggerableDelay 0.05)
      (CallFunction|StopRecoil))))

(event Custom|FireRateCalculate
  ;[0.03876 0.002488 0.08333 1 12] Fire rate for non automatic weapons
  (Variables|/Game/FPSGame/Character/BP_FP_Player.BP_FP_Player_C|SetIsWeaponFireLoading? (Variables|Default|GetPlayer) true)
  (Utilities|FlowControl|Delay (Variables|Shotgun|GetFireRate))
  (Variables|/Game/FPSGame/Character/BP_FP_Player.BP_FP_Player_C|SetIsWeaponFireLoading? (Variables|Default|GetPlayer) false))

(event Custom|WeaponAimEnter
  ;[0 1 0.625] Binds aiming bool to ADS input action on BP_FP_Player
  (Variables|Default|SetIsAimingWeapon? true))

(event Custom|WeaponAimExit
  ;[0 1 0.625] Binds aiming bool to ADS input action on BP_FP_Player
  (Variables|Default|SetIsAimingWeapon? false))

(event EventBeginPlay
  ;[0 0.2734 1 1 12] Reference to Player
  (bind _asbp_fp_player (Utilities|Casting|CastToBP_FP_Player (Game|GetPlayerCharacter 0)))
  (bind _output_get (Variables|Default|SetPlayer _asbp_fp_player))
  ;[0 1 0.625] Binds aiming bool to ADS input action on BP_FP_Player
  (Variables|AmmoData|SetIsCurrentAmmoFull? (== (Variables|AmmoData|GetCurrentAmmo) (Variables|AmmoData|GetMagazineSize)))
  (EventDispatchers|BindEventtoAimEnter _output_get (delegate Custom|WeaponAimEnter))
  (EventDispatchers|BindEventtoAimExit _output_get (delegate Custom|WeaponAimExit)))

(fn ConstructionScript)

(fn AmmoPickup
  (params (AmmoType :type E_AmmoType%20Enum :default "NewEnumerator0"))
  (switch Utilities|FlowControl|Switch|SwitchonE_AmmoType AmmoType
    (:NewEnumerator0
      ;[0.07812 1 0 1 12] Adds ammo if pistol is picking up pistol ammo
      (if (Utilities|Enum|Equal(Enum) (Variables|WeaponData|GetWeaponType) "NewEnumerator0")
        (Variables|AmmoData|SetCurrentTotalAmmo (+ (Variables|AmmoPickups|GetPistolPickupAmount) (Variables|AmmoData|GetCurrentTotalAmmo)))
        (return true)
        (else
          (return false))))
    (:NewEnumerator1
      ;[0.07812 1 0 1 12] Adds ammo if pistol is picking up pistol ammo
      (if (Utilities|Enum|Equal(Enum) (Variables|WeaponData|GetWeaponType) "NewEnumerator1")
        (Variables|AmmoData|SetCurrentTotalAmmo (+ (Variables|AmmoPickups|GetRiflePickupAmount) (Variables|AmmoData|GetCurrentTotalAmmo)))
        (return true)
        (else
          (return false))))
    (:NewEnumerator2
      ;[0.07812 1 0 1 12] Adds ammo if shotgun is picking up shotgun ammo
      (if (Utilities|Enum|Equal(Enum) (Variables|WeaponData|GetWeaponType) "NewEnumerator2")
        (Variables|AmmoData|SetCurrentTotalAmmo (+ (Variables|AmmoPickups|GetShotgunPickupAmount) (Variables|AmmoData|GetCurrentTotalAmmo)))
        (return true)
        (else
          (return false))))
    (:NewEnumerator3
      ;[0.07812 1 0 1 12] Adds ammo if sniper rifle is picking up sniper ammo
      (if (Utilities|Enum|Equal(Enum) (Variables|WeaponData|GetWeaponType) "NewEnumerator3")
        (Variables|AmmoData|SetCurrentTotalAmmo (+ (Variables|AmmoPickups|GetSniperPickupAmount) (Variables|AmmoData|GetCurrentTotalAmmo)))
        (return true)
        (else
          (return false))))
    (:NewEnumerator4
      ;[0.07812 1 0 1 12] Adds ammo if grenade launcher is picking up grenade ammo
      (if (Utilities|Enum|Equal(Enum) (Variables|WeaponData|GetWeaponType) "NewEnumerator4")
        (Variables|AmmoData|SetCurrentTotalAmmo (+ (Variables|AmmoPickups|GetGrenadePickupAmount) (Variables|AmmoData|GetCurrentTotalAmmo)))
        (return true)
        (else
          (return false))))
    (:NewEnumerator5
      ;[0.07812 1 0 1 12] Adds ammo if rocket launcher is picking up rocket ammo
      (if (Utilities|Enum|Equal(Enum) (Variables|WeaponData|GetWeaponType) "NewEnumerator5")
        (Variables|AmmoData|SetCurrentTotalAmmo (+ (Variables|AmmoPickups|GetRocketPickupAmount) (Variables|AmmoData|GetCurrentTotalAmmo)))
        (return true)
        (else
          (return false))))))

(fn StartShooting
  (params (Firetype :type E-Firetype%20Enum :default "NewEnumerator0"))
  (Utilities|FlowControl|Sequence
    (:then_0
      ;[1 0.3516 0 1 12] Subtracts a bullet when firing
      (Variables|AmmoData|SetCurrentAmmo (- (Variables|AmmoData|GetCurrentAmmo) 1))
      ;[0.6172 0 1 1 12] Set flag to false
      (Variables|AmmoData|SetIsCurrentAmmoFull? false)
      ;[0 0.9766 1 1 12] Auto reload gun whem mag becomes empty
      (if (<= (Variables|AmmoData|GetCurrentAmmo) 0)
        (CallFunction|AutoReloadonEmpty)))
    (:then_1
      (switch Utilities|FlowControl|Switch|SwitchonE-Firetype Firetype
        (:NewEnumerator0
          (if (Variables|Shotgun|GetIsShotgun?)
            (for _index (range 0 (- (Variables|Shotgun|GetPelletCount) 1)) ; Shoots extra lin traces
              ;[0.1667 0.0127 0.03098 1 12] Draw line trace for hitscan weapons
              (bind _hitresult (CallFunction|CalculateLineTrace (Variables|/Game/FPSGame/Character/BP_FP_Player.BP_FP_Player_C|GetCamera (Variables|Default|GetPlayer)) (Variables|Default|GetWeaponMesh) (Variables|WeaponData|GetWeapon%20Socket)))
              (CallFunction|AddDamage)
              (Game|SpawnActorfromClass (Variables|Default|GetImpactEffect) (Math|Transform|MakeTransform (.ImpactPoint (Collision|BreakHitResult _hitresult)) "0, 0, 0" "1,1,1") "Undefined" 0 _hitresult 0)
              (CallFunction|StartRecoil)
              (Variables|WeaponData|SetIsFiring? true))
            (else
              (bind _hitresult_2 (CallFunction|CalculateLineTrace (Variables|/Game/FPSGame/Character/BP_FP_Player.BP_FP_Player_C|GetCamera (Variables|Default|GetPlayer)) (Variables|Default|GetWeaponMesh) (Variables|WeaponData|GetWeapon%20Socket)))
              (CallFunction|AddDamage)
              (Game|SpawnActorfromClass (Variables|Default|GetImpactEffect) (Math|Transform|MakeTransform (.ImpactPoint (Collision|BreakHitResult _hitresult_2)) "0, 0, 0" "1,1,1") "Undefined" 0 _hitresult_2 0)
              (CallFunction|StartRecoil)
              (Variables|WeaponData|SetIsFiring? true))))))))

(fn CalculateLineTrace
  (params (Camera :type Camera%20Component%20Object%20Reference) (WeaponMesh :type Scene%20Component%20Object%20Reference) (WeaponSocket :type Text))
  (bind _bulletspread (Variables|AmmoData|GetBulletSpread))
  (bind _returnvalue (* _bulletspread -1.0))
  (Utilities|FlowControl|Sequence
    (:then_0
      (LocalVariables|SetLocalCamera Camera))
    (:then_1
      (bind _outhit (Collision|LineTraceForObjects (.location (Transformation|GetWorldTransform (LocalVariables|GetLocalCamera))) (select (Variables|/Game/FPSGame/Character/BP_FP_Player.BP_FP_Player_C|GetIsAiming? (Variables|Default|GetPlayer)) (+ (.location (Transformation|GetWorldTransform (LocalVariables|GetLocalCamera))) (* (Math|Vector|GetForwardVector (.rotation (Transformation|GetWorldTransform (LocalVariables|GetLocalCamera)))) (Variables|WeaponData|GetLineTraceDistance))) (Math|Vector|MakeVector (+ (.X (Math|Vector|BreakVector (+ (.location (Transformation|GetWorldTransform (LocalVariables|GetLocalCamera))) (* (Math|Vector|GetForwardVector (.rotation (Transformation|GetWorldTransform (LocalVariables|GetLocalCamera)))) (Variables|WeaponData|GetLineTraceDistance))))) (Math|Random|RandomFloatinRange _returnvalue _bulletspread)) (+ (.Y (Math|Vector|BreakVector (+ (.location (Transformation|GetWorldTransform (LocalVariables|GetLocalCamera))) (* (Math|Vector|GetForwardVector (.rotation (Transformation|GetWorldTransform (LocalVariables|GetLocalCamera)))) (Variables|WeaponData|GetLineTraceDistance))))) (Math|Random|RandomFloatinRange _returnvalue _bulletspread)) (+ (.Z (Math|Vector|BreakVector (+ (.location (Transformation|GetWorldTransform (LocalVariables|GetLocalCamera))) (* (Math|Vector|GetForwardVector (.rotation (Transformation|GetWorldTransform (LocalVariables|GetLocalCamera)))) (Variables|WeaponData|GetLineTraceDistance))))) (Math|Random|RandomFloatinRange _returnvalue _bulletspread)))) (Utilities|Array|MakeArray "ObjectTypeQuery1" "ObjectTypeQuery2" "ObjectTypeQuery3") false (Utilities|Array|MakeArray (Game|GetPlayerCharacter 0)) "None" true "(R=1.000000,G=0.000000,B=0.000000,A=1.000000)" "(R=0.000000,G=1.000000,B=0.000000,A=1.000000)" 1e+01)))
    (:then_2
      (return _outhit))))

(fn ReloadCalculation
  (bind _output_get (Variables|AmmoData|SetBulletDifference (- (Variables|AmmoData|GetMagazineSize) (Variables|AmmoData|GetCurrentAmmo))))
  (if (<= _output_get (Variables|AmmoData|GetCurrentTotalAmmo))
    ;[0.07399 0.1069 0.1719 1 12] Runs when there is reserve ammo
    (Variables|AmmoData|SetCurrentAmmo (Variables|AmmoData|GetMagazineSize))
    (Variables|AmmoData|SetCurrentTotalAmmo (- (Variables|AmmoData|GetCurrentTotalAmmo) (Variables|AmmoData|GetBulletDifference)))
    (else
      ;[0 0.1562 1 1 12] Runs when reserve amount is lower than the ammo in the magazine
      (Variables|AmmoData|SetCurrentAmmo (+ (Variables|AmmoData|GetCurrentAmmo) (Variables|AmmoData|GetCurrentTotalAmmo)))
      (Variables|AmmoData|SetCurrentTotalAmmo 0))))

(fn IsMagFullorEmpty
  (if (== (Variables|AmmoData|GetCurrentAmmo) (Variables|AmmoData|GetMagazineSize))
    _
    (elif (== (Variables|AmmoData|GetCurrentTotalAmmo) 0)
      _
      (else
        ;[0.6867 0 1 1 12] Enables reload if mag is empty but ammo in reserves
        (bind _output_get (Variables|/Game/FPSGame/Character/BP_FP_Player.BP_FP_Player_C|SetCanReload? (Variables|Default|GetPlayer) true))
        (return _output_get))))
  ;[0.6867 0 1 1 12] Disables reload if mag is full or reserves are empty
  (bind _output_get_2 (Variables|/Game/FPSGame/Character/BP_FP_Player.BP_FP_Player_C|SetCanReload? (Variables|Default|GetPlayer) false))
  (return _output_get_2))

(fn DoWeHaveAmmo?
  ;[0 1 0.7656 1 12] Allows shoot event to occur if player has ammo.
  (return (> (Variables|AmmoData|GetCurrentAmmo) 0)))

(fn IsThereAmmoLeft?
  ;[0.6867 0 1 1 12] Check for ammo in reserve
  (return (> (Variables|AmmoData|GetCurrentTotalAmmo) 0)))

(fn StopShooting
  (Variables|WeaponData|SetIsFiring? false))

(fn ShotgunReloadPellets
  (Variables|WeaponData|SetReloadTime (* (- (Variables|AmmoData|GetMagazineSize) (Variables|AmmoData|GetCurrentAmmo)) (Variables|WeaponData|GetReloadTime))))

(fn HowManyShellstoReload
  (Variables|AmmoData|SetBulletDifference (- (Variables|AmmoData|GetMagazineSize) (Variables|AmmoData|GetCurrentAmmo))))

(fn IsReserveAmmoSufficient?
  (if (!= (Variables|AmmoData|GetCurrentTotalAmmo) 0)
    (if (<= (Variables|AmmoData|GetBulletDifference) (Variables|AmmoData|GetCurrentTotalAmmo))
      (bind _output_get (Variables|AmmoData|SetReserveAmmoSufficient? true))
      (return _output_get)
      (else
        (Variables|AmmoData|SetBulletDifference (Variables|AmmoData|GetCurrentTotalAmmo))
        (bind _output_get_2 (Variables|AmmoData|SetReserveAmmoSufficient? true))
        (return _output_get_2)))
    (else
      (bind _output_get_3 (Variables|AmmoData|SetReserveAmmoSufficient? false))
      (return _output_get_3))))

(fn LoadShotgunShell
  (if (not (== (Variables|AmmoData|GetCurrentAmmo) (Variables|AmmoData|GetMagazineSize)))
    (Math|Integer|DecrementInt (Variables|AmmoData|GetCurrentTotalAmmo)
      (:%20%20
        (Math|Integer|DecrementInt (Variables|AmmoData|GetBulletDifference)
          (:%20%20
            (Math|Integer|IncrementInt (Variables|AmmoData|GetCurrentAmmo)
              (:%20%20
                (if (== (Variables|AmmoData|GetCurrentAmmo) (Variables|AmmoData|GetMagazineSize))
                  (bind _output_get (Variables|AmmoData|SetIsCurrentAmmoFull? true))
                  (return _output_get)
                  (else
                    (bind _output_get_2 (Variables|AmmoData|SetIsCurrentAmmoFull? false))
                    (return _output_get_2)))))))))))

(fn AddDamage
  (params (HitResult :type Hit%20Result%20Structure))
  ;[0 0.03513 0.3177 1 12] Passes info thru weapon  to enemy taking damage
  (Class|BPITakeDamage|EnemyTakeDamage(Message) (.HitActor (Collision|BreakHitResult HitResult)) (Variables|Default|GetWeaponStats) HitResult))