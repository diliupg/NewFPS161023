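; BP_SniperRifle is a sniper rifle weapon that extends a parent weapon's shooting and aiming behavior.
; Firing plays the rifle's fire animation on the weapon mesh and runs the fire rate calculation.
; Aiming, when it is the player's current weapon, shows a scope crosshair widget while hiding the weapon mesh, player character and main HUD.
; Leaving aim removes the widget and restores their visibility.
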(event EventStartShooting
  (params (Firetype :type E-Firetype%20Enum :default "NewEnumerator0"))
  (|CallParentFunction Firetype)
  (Components|Animation|PlayAnimation (Variables|Default|GetWeaponMesh) "/Game/WeaponMeshes/MilitaryWeapSilver/Weapons/Animations/Fire_SniperRifle_W.Fire_SniperRifle_W" false)
  (CallFunction|FireRateCalculate))

(event EventWeaponAimEnter
  (|CallParentFunction)
  (if (== (Variables|/Game/FPSGame/Character/BP_FP_Player.BP_FP_Player_C|GetCurrentWeapon (Variables|Default|GetPlayer)) self)
    (bind _returnvalue (UserInterface|CreateWidget "/Game/FPSGame/UI/SnipeRifleCrosshairs.SnipeRifleCrosshairs_C"))
    ;[1 0.1655 0.5038 1 12] Adds widget to viewport ONLY if it is not there.
    (if (not (UserInterface|Viewport|IsinViewport _returnvalue))
      (UserInterface|Viewport|AddtoViewport _returnvalue 0)
      ;[0.1375 0.2402 1 1 12] Hides player, weapon and HUD while  sniper aiming
      (Development|SetHiddeninGame (Variables|Default|GetWeaponMesh) true false)
      (Rendering|SetActorHiddenInGame (Game|GetPlayerCharacter 0) true)
      (Widget|SetVisibility (Variables|/Game/FPSGame/Character/BP_FP_Player.BP_FP_Player_C|GetMainHUD (Variables|Default|GetPlayer)) "Collapsed"))))

(event EventWeaponAimExit
  (|CallParentFunction)
  (Utilities|IsValid (stale EventWeaponAimEnter _returnvalue)
    (:Is%20Valid
      (Widget|RemovefromParent (stale EventWeaponAimEnter _returnvalue))
      ;[0.2455 0.3493 0.8229 1 12] Unhides weapon, player, and HUD while sniper aiming
      (Development|SetHiddeninGame (Variables|Default|GetWeaponMesh) false false)
      (Rendering|SetActorHiddenInGame (Game|GetPlayerCharacter 0) false)
      (Widget|SetVisibility (Variables|/Game/FPSGame/Character/BP_FP_Player.BP_FP_Player_C|GetMainHUD (Variables|Default|GetPlayer)) "Visible"))))

(fn ConstructionScript
  (|CallParentFunction))