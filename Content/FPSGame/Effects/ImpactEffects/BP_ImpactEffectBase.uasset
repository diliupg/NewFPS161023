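; Base impact effect actor for the FPS game that plays surface-specific feedback at a stored hit result when it begins play.
; On a blocking hit, it picks a particle, sound and decal from the physical material's surface type, with body parts sharing flesh effects.
; The decal aligns to the impact normal with random roll and attaches to the hit component and bone for a set lifespan.
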(event EventBeginPlay
  (bind _hiresult (Variables|Default|GetHiResult))
  (bind _stonefx (Variables|Default|GetStoneFX))
  (bind _fleshimpactdecal (Variables|Default|GetFleshImpactDecal))
  (bind _hiresult_2 (Variables|Default|GetHiResult))
  (bind _hiresult_3 (Variables|Default|GetHiResult))
  (bind _bodysfx (Variables|Default|GetBodySFX))
  (bind _stonesfx (Variables|Default|GetStoneSFX))
  (bind _stoneimpactdecal (Variables|Default|GetStoneImpactDecal))
  (bind _decalsize (Variables|Default|GetDecalSize))
  (bind _hiresult_4 (Variables|Default|GetHiResult))
  (bind _bodyfx (Variables|Default|GetBodyFX))
  (bind _impactnormal (Collision|BreakHitResult _hiresult))
  (bind (_bblockinghit _binitialoverlap _time _distance _location _impactpoint _normal _impactnormal_2 _physmat) (Collision|BreakHitResult _hiresult_3))
  (bind (_bblockinghit_2 _binitialoverlap_2 _time_2 _distance_2 _location_2 _impactpoint_2 _normal_2 _impactnormal_3 _physmat_2) (Collision|BreakHitResult _hiresult_4))
  (bind (_bblockinghit_3 _binitialoverlap_3 _time_3 _distance_3 _location_3 _impactpoint_3 _normal_3 _impactnormal_4 _physmat_3 _hitactor _hitcomponent _hitbonename) (Collision|BreakHitResult _hiresult_2))
  (bind _returnvalue (Math|Conversions|RotationFromXVector _impactnormal))
  (bind (_roll _pitch _yaw) (Math|Rotator|BreakRotator _returnvalue))
  (Utilities|FlowControl|Sequence
    (:then_0
      (if _bblockinghit_2
        ;[0.1596 0.1271 0.5 1 12] Particle effects for different surface types
        (Effects|SpawnEmitteratLocation (Utilities|Select :Index (Variables|/Script/PhysicsCore.PhysicalMaterial|GetSurfaceType _physmat_2) :SurfaceType_Default _stonefx :SurfaceType1 _bodyfx :SurfaceType2 _bodyfx :SurfaceType3 _bodyfx :SurfaceType4 (Variables|Default|GetMetalFX) :SurfaceType5 _stonefx :SurfaceType6 (Variables|Default|GetGlassFX) :SurfaceType7 (Variables|Default|GetConcreteFX) :SurfaceType8 (Variables|Default|GetWoodFX) :SurfaceType9 0) _impactpoint_2)))
    (:then_1
      (if _bblockinghit
        ;[0.05131 0 0.06771 1 12] Sound effects for different surface types
        (Audio|PlaySoundatLocation (Utilities|Select :Index (Variables|/Script/PhysicsCore.PhysicalMaterial|GetSurfaceType _physmat) :SurfaceType_Default _stonesfx :SurfaceType1 _bodysfx :SurfaceType2 _bodysfx :SurfaceType3 _bodysfx :SurfaceType4 (Variables|Default|GetMetalSFX) :SurfaceType5 _stonesfx :SurfaceType6 (Variables|Default|GetGlassSFX) :SurfaceType7 (Variables|Default|GetConcreteSFX) :SurfaceType8 (Variables|Default|GetWoodSFX) :SurfaceType9 0) _impactpoint "0, 0, 0" 1.0 1.0 0.0 0 0 0)))
    (:then_2
      ;[0 0.4375 1 1 12] Randomize decal rotation
      (Variables|Default|SetDecalRotation (Math|Rotator|MakeRotator (Math|Random|RandomFloatinRange -1.8e+02 1.8e+02) _pitch _yaw)))
    (:then_3
      (if _bblockinghit_3
        ;[0.1667 0.026 0.08235 1 12] Decals
        (Class|GameplayStatics|SpawnDecalAttached (Utilities|Select :Index (Variables|/Script/PhysicsCore.PhysicalMaterial|GetSurfaceType _physmat_3) :SurfaceType_Default _stoneimpactdecal :SurfaceType1 _fleshimpactdecal :SurfaceType2 _fleshimpactdecal :SurfaceType3 _fleshimpactdecal :SurfaceType4 0 :SurfaceType5 _stoneimpactdecal :SurfaceType6 (Variables|Default|GetGlassImpactDecal) :SurfaceType7 (Variables|Default|GetConcretempactDecal) :SurfaceType8 (Variables|Default|GetWoodImpactDecal) :SurfaceType9 0) (Math|Vector|MakeVector _decalsize _decalsize _decalsize) _hitcomponent _hitbonename _impactpoint_3 (Variables|Default|GetDecalRotation) "KeepWorldPosition" (Variables|Default|GetDecalLifespan))))))

(fn ConstructionScript)