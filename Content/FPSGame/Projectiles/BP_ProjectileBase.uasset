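; Base projectile that applies direct or radial damage on impact and expires after a set lifespan.
; At spawn it takes the player's CurrentVelocity when the GrenadePathAI flag is set, then clears the flag.
; On stop it sends damage interface messages to the hit actor, plus sphere-overlapped actors and an impulse actor for radial damage.
; It then hides the mesh, spawns an impact effect and destroys itself after a short delay.
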(event OnProjectileStop(ProjectileMovement)
  (params (ImpactResult :type Hit%20Result%20Structure%20%28by%20ref%29))
  (CallFunction|StopProjectile ImpactResult))

(event EventBeginPlay
  ;[0 0.8359 1 1 12] Reference to player
  (bind _asbp_fp_player (Utilities|Casting|CastToBP_FP_Player (Game|GetPlayerCharacter 0)))
  (Variables|Default|SetPlayer _asbp_fp_player)
  ;[0.1406 0.01112 0.09238 1 12] Set the Projectile velocity
  (if (Variables|/Game/FPSGame/Character/BP_FP_Player.BP_FP_Player_C|GetGrenadePathAI (Variables|Default|GetPlayer))
    (Variables|/Script/Engine.MovementComponent|SetVelocity (Variables|Default|GetProjectileMovement) (Variables|/Game/FPSGame/Character/BP_FP_Player.BP_FP_Player_C|GetCurrentVelocity (Variables|Default|GetPlayer)))
    (Variables|/Game/FPSGame/Character/BP_FP_Player.BP_FP_Player_C|SetGrenadePathAI (Variables|Default|GetPlayer) false))
  ;;[0.6545 1 0.2493 1 12] Projectile is taken out of the game whether it hits anything or not
  (Actor|SetLifeSpan (Variables|Default|GetLifespan)))

(fn ConstructionScript)

(fn StopProjectile
  (params (HitResult :type Hit%20Result%20Structure))
  (bind (_bblockinghit _binitialoverlap _time _distance _location _impactpoint _normal _impactnormal _physmat _hitactor) (Collision|BreakHitResult HitResult))
  (bind _projectilemesh (Variables|Default|GetProjectileMesh))
  (bind _weaponstats (Variables|Default|GetWeaponStats))
  (bind (_damage _impactradius) (Utilities|Struct|BreakS_WeaponStats _weaponstats))
  (bind _s_damageinfo (Utilities|Struct|MakeS_DamageInfo _damage "NewEnumerator2"))
  (Utilities|FlowControl|Sequence
    (:then_0
      (if (Variables|Default|GetIsDealingRadialDamage?)
        (CallFunction|ExplodeProjectile HitResult)
        ;[1 0.1562 0.1822 1 14] On each actor hit
        (Class|BPIDamageble|TakeRadialDamageBPID(Message) _hitactor _s_damageinfo self _impactradius _impactpoint)
        (else
          (Class|BPIDamageble|TakeDamageBPID(Message) _hitactor _s_damageinfo))))
    (:then_1
      ;[0 0.1562 1 1 12] Removes mesh, spawns impact effect, destroys actor after delay
      ;;[0.5 0.5 0.5] Set New Hidden to true
      (Development|SetHiddeninGame _projectilemesh true false)
      (Game|SpawnActorfromClass (Variables|Default|GetImpactEffect) (Transformation|GetWorldTransform _projectilemesh) "AlwaysSpawn" 0 HitResult 0)
      (Actor|SetLifeSpan 1.0))))

(fn ExplodeProjectile
  (params (HitResult :type Hit%20Result%20Structure))
  (bind _impactpoint (Collision|BreakHitResult HitResult))
  (bind _weaponstats (Variables|Default|GetWeaponStats))
  (bind (_damage _impactradius) (Utilities|Struct|BreakS_WeaponStats _weaponstats))
  (Utilities|FlowControl|Sequence
    (:then_0
      (bind _outactors (Collision|SphereOverlapActors _impactpoint _impactradius (Utilities|Array|MakeArray "ObjectTypeQuery2" "ObjectTypeQuery3") 0))
      (for _array_element _outactors
        (Class|BPIDamageble|TakeRadialDamageBPID(Message) _array_element (Utilities|Struct|MakeS_DamageInfo _damage "NewEnumerator2") self _impactradius _impactpoint)))
    (:then_1
      (Game|SpawnActorfromClass "/Game/FPSGame/Projectiles/ExplosionImpulse.ExplosionImpulse_C" (Math|Transform|MakeTransform _impactpoint "0, 0, 0" "1,1,1") "AlwaysSpawn" 0 0))))