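; Placeable minimap custom area: a box or cylinder trigger volume that reports the player and minimap-tagged actors entering or leaving it to the attached minimap.
; The construction script shows and sizes the chosen shape, and Activate stores the minimap and enables that shape's query collision.
; Overlap events track tagged actors and have the minimap re-evaluate its custom areas.
; Helper functions query which minimap detector objects are inside.
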(event OnComponentBeginOverlap(Box_Trigger)
  (params (OverlappedComponent :type Primitive%20Component%20Object%20Reference) (OtherActor :type Actor%20Object%20Reference) (OtherComp :type Primitive%20Component%20Object%20Reference) (OtherBodyIndex :type Integer) (bFromSweep :type Boolean) (SweepResult :type Hit%20Result%20Structure%20%28by%20ref%29))
  ;[1 1 1] When player enters trigger, tell the minimap to update its custom areas and check if this is the first trigger entered.
  ; When a minimap actor enters trigger, add to stored list of actors, and tell the minimap to check if this is the first trigger entered.
  (if (== OtherActor (Game|GetPlayerCharacter 0))
    (Default|UpdateCustomAreas (Variables|DO_NOT_EDIT|GetINTERNAL_AttachedMinimap) true)
    (elif (Actor|ActorHasTag OtherActor "MinimapCollision")
      (Utilities|Array|Add (Variables|DO_NOT_EDIT|GetINTERNAL_ActorsEntered) OtherActor)
      (Default|CheckActorJustEnteredCustomArea (Variables|DO_NOT_EDIT|GetINTERNAL_AttachedMinimap) OtherActor))))

(event OnComponentBeginOverlap(CylinderMesh_Trigger)
  (params (OverlappedComponent :type Primitive%20Component%20Object%20Reference) (OtherActor :type Actor%20Object%20Reference) (OtherComp :type Primitive%20Component%20Object%20Reference) (OtherBodyIndex :type Integer) (bFromSweep :type Boolean) (SweepResult :type Hit%20Result%20Structure%20%28by%20ref%29))
  ;[1 1 1] When player enters trigger, tell the minimap to update its custom areas and check if this is the first trigger entered.
  ; When a minimap actor enters trigger, add to stored list of actors, and tell the minimap to check if this is the first trigger entered.
  (if (== OtherActor (Game|GetPlayerCharacter 0))
    (Default|UpdateCustomAreas (Variables|DO_NOT_EDIT|GetINTERNAL_AttachedMinimap) true)
    (elif (Actor|ActorHasTag OtherActor "MinimapCollision")
      (Utilities|Array|Add (Variables|DO_NOT_EDIT|GetINTERNAL_ActorsEntered) OtherActor)
      (Default|CheckActorJustEnteredCustomArea (Variables|DO_NOT_EDIT|GetINTERNAL_AttachedMinimap) OtherActor))))

(event OnComponentEndOverlap(Box_Trigger)
  (params (OverlappedComponent :type Primitive%20Component%20Object%20Reference) (OtherActor :type Actor%20Object%20Reference) (OtherComp :type Primitive%20Component%20Object%20Reference) (OtherBodyIndex :type Integer))
  ;[1 1 1] When player exits trigger, tell the minimap to update its custom areas and check if the player has exited ALL of them.
  ; When a minimap actor exits trigger, remove from stored list of actors, and check the minimap if it has exited ALL custom areas.
  (if (== OtherActor (Game|GetPlayerCharacter 0))
    (Default|UpdateCustomAreas (Variables|DO_NOT_EDIT|GetINTERNAL_AttachedMinimap) false)
    (elif (Actor|ActorHasTag OtherActor "MinimapCollision")
      (if (Utilities|Array|ContainsItem (Variables|DO_NOT_EDIT|GetINTERNAL_ActorsEntered) OtherActor)
        (Utilities|Array|RemoveItem (Variables|DO_NOT_EDIT|GetINTERNAL_ActorsEntered) OtherActor)
        (Default|CheckHasJustExitedCustomArea (Variables|DO_NOT_EDIT|GetINTERNAL_AttachedMinimap) OtherActor)))))

(event OnComponentEndOverlap(CylinderMesh_Trigger)
  (params (OverlappedComponent :type Primitive%20Component%20Object%20Reference) (OtherActor :type Actor%20Object%20Reference) (OtherComp :type Primitive%20Component%20Object%20Reference) (OtherBodyIndex :type Integer))
  ;[1 1 1] When player exits trigger, tell the minimap to update its custom areas and check if the player has exited ALL of them.
  ; When a minimap actor exits trigger, remove from stored list of actors, and check the minimap if it has exited ALL custom areas.
  (if (== OtherActor (Game|GetPlayerCharacter 0))
    (Default|UpdateCustomAreas (Variables|DO_NOT_EDIT|GetINTERNAL_AttachedMinimap) false)
    (elif (Actor|ActorHasTag OtherActor "MinimapCollision")
      (if (Utilities|Array|ContainsItem (Variables|DO_NOT_EDIT|GetINTERNAL_ActorsEntered) OtherActor)
        (Utilities|Array|RemoveItem (Variables|DO_NOT_EDIT|GetINTERNAL_ActorsEntered) OtherActor)
        (Default|CheckHasJustExitedCustomArea (Variables|DO_NOT_EDIT|GetINTERNAL_AttachedMinimap) OtherActor)))))

(event Custom|Activate
  (params (Minimap :type BP%20Minimap%20Object%20Reference))
  ;[1 1 1] On activation, turn on the collision trigger depending on the shape
  (Variables|DO_NOT_EDIT|SetINTERNAL_AttachedMinimap Minimap)
  (switch Utilities|FlowControl|Switch|SwitchonENUM_MinimapCustomTriggerShape (Variables|Default|GetShape)
    (:NewEnumerator0
      (Collision|SetCollisionEnabled (Variables|Default|GetBox_Trigger) "QueryOnly"))
    (:NewEnumerator1
      (Collision|SetCollisionEnabled (Variables|Default|GetCylinderMesh_Trigger) "QueryOnly"))))

(fn ConstructionScript
  ;[1 1 1] Update the size of the trigget box/cylinder
  (switch Utilities|FlowControl|Switch|SwitchonENUM_MinimapCustomTriggerShape (Variables|Default|GetShape)
    (:NewEnumerator0
      (Rendering|SetVisibility (Variables|Default|GetCylinderMesh_Trigger) false true)
      (Rendering|SetVisibility (Variables|Default|GetBox_Trigger) true true)
      (Components|Box|SetBoxExtent (Variables|Default|GetBox_Trigger) (* (Variables|Default|GetSize) 0.5) true)
      (Transformation|SetWorldScale3D (Variables|Default|GetCubeMesh_ForDisplayInEditorOnly) (/ (Variables|Default|GetSize) 1e+02)))
    (:NewEnumerator1
      (Rendering|SetVisibility (Variables|Default|GetBox_Trigger) false true)
      (Rendering|SetVisibility (Variables|Default|GetCylinderMesh_Trigger) true true)
      (Transformation|SetWorldScale3D (Variables|Default|GetCylinderMesh_Trigger) (/ (Variables|Default|GetSize) 1e+02)))))

(fn IsActorInsideRegion
  (params (Actor :type Actor%20Object%20Reference))
  ;[1 1 1] Check if the supplied actor is inside this minimap custom area.
  (switch Utilities|FlowControl|Switch|SwitchonENUM_MinimapCustomTriggerShape (Variables|Default|GetShape)
    (:NewEnumerator0
      (return (Utilities|Array|ContainsItem (Collision|GetOverlappingActors (Variables|Default|GetBox_Trigger) "/Game/Minimap/Blueprints/BP_MinimapDetectorAttachmentObject.BP_MinimapDetectorAttachmentObject_C" :!class /Script/Engine.PrimitiveComponent) Actor)))
    (:NewEnumerator1
      (return (Utilities|Array|ContainsItem (Collision|GetOverlappingActors (Variables|Default|GetCylinderMesh_Trigger) "/Game/Minimap/Blueprints/BP_MinimapDetectorAttachmentObject.BP_MinimapDetectorAttachmentObject_C" :!class /Script/Engine.PrimitiveComponent) Actor)))))

(fn GetAllOverlappingActors
  ;[1 1 1] Get all minimap actors that are currently inside this custom minimap area.
  (switch Utilities|FlowControl|Switch|SwitchonENUM_MinimapCustomTriggerShape (Variables|Default|GetShape)
    (:NewEnumerator0
      (return (Collision|GetOverlappingActors (Variables|Default|GetBox_Trigger) "/Game/Minimap/Blueprints/BP_MinimapDetectorAttachmentObject.BP_MinimapDetectorAttachmentObject_C" :!class /Script/Engine.PrimitiveComponent)))
    (:NewEnumerator1
      (return (Collision|GetOverlappingActors (Variables|Default|GetCylinderMesh_Trigger) "/Game/Minimap/Blueprints/BP_MinimapDetectorAttachmentObject.BP_MinimapDetectorAttachmentObject_C" :!class /Script/Engine.PrimitiveComponent)))))