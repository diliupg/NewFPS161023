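; Placeable minimap volume that configures and drives the shared Widget_Minimap while the player is inside its box or linked custom areas.
; Overlapping volumes are tracked in a SortOrder-ranked stack on each minimap, so the highest takes over and another resumes on exit.
; A shared bounds trigger, attached to the player or volume, gates nearby icons, while off-screen-tracked icons register on activation.
; A looping timer retries initialisation until dependencies are valid.
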(event OnComponentBeginOverlap(MinimapVolume_Trigger)
  (params (OverlappedComponent :type Primitive%20Component%20Object%20Reference) (OtherActor :type Actor%20Object%20Reference) (OtherComp :type Primitive%20Component%20Object%20Reference) (OtherBodyIndex :type Integer) (bFromSweep :type Boolean) (SweepResult :type Hit%20Result%20Structure%20%28by%20ref%29))
  ;[1 1 1] Default Trigger Volume
  ;[1 1 1] If the actor entered is the player, attempt to enable this minimap
  (if (== OtherActor (Game|GetPlayerCharacter 0))
    (CallFunction|AttemptEnableMinimap)
    (else
      ;[1 1 1] If actor is a valid minimap object and just has entered
      ;  this minimap volume, display it on the minimap
      (if (Variables|DO_NOT_EDIT|GetINTERNAL_CurrentlyActive)
        (if (Actor|ActorHasTag OtherActor "MinimapCollision")
          (if (Default|IsOverlapping (Variables|DO_NOT_EDIT|GetINTERNAL_MinimapBoundsTrigger) OtherActor)
            (Default|AddActortoShow (Variables|DO_NOT_EDIT|GetINTERNAL_MinimapWidget) (Actor|GetComponentbyClass (Actor|GetAttachParentActor OtherActor) "/Game/DynamicMinimapSystem/Blueprints/Component_MinimapIcon.Component_MinimapIcon_C"))))))))

(event OnComponentEndOverlap(MinimapVolume_Trigger)
  (params (OverlappedComponent :type Primitive%20Component%20Object%20Reference) (OtherActor :type Actor%20Object%20Reference) (OtherComp :type Primitive%20Component%20Object%20Reference) (OtherBodyIndex :type Integer))
  ;[1 1 1] Default Trigger Volume
  ;[1 1 1] If the actor exited is the player, disable this minimap
  (if (== OtherActor (Game|GetPlayerCharacter 0))
    (CallFunction|DisableMinimap true true)
    (else
      ;[1 1 1] If actor is a valid minimap object and just has exited
      ;  this minimap volume, remove it from the minimap
      (if (Variables|DO_NOT_EDIT|GetINTERNAL_CurrentlyActive)
        (if (Actor|ActorHasTag OtherActor "MinimapCollision")
          (Default|RemoveActortoShow (Variables|DO_NOT_EDIT|GetINTERNAL_MinimapWidget) (Actor|GetComponentbyClass (Actor|GetAttachParentActor OtherActor) "/Game/DynamicMinimapSystem/Blueprints/Component_MinimapIcon.Component_MinimapIcon_C")))))))

(event Custom|AttemptToInitialise
  ;[1 1 1] Keep checking if everything required is initialised.
  ; Clear timer when initialisation successful.
  (bind _isinitialised (CallFunction|AttemptInitialisation))
  (if _isinitialised
    (Variables|DO_NOT_EDIT|SetINTERNAL_IsInitialised true)
    (Utilities|Time|ClearandInvalidateTimerbyHandle (Variables|DO_NOT_EDIT|GetINTERNAL_CheckMinimapValidTimer))))

(event Custom|PushMinimapToStack
  (params (Minimap :type BP%20Minimap%20Object%20Reference))
  ;[1 1 1] Adds and removes minimaps from the stack
  (Utilities|Array|Add (Variables|DO_NOT_EDIT|GetINTERNAL_MinimapStack) Minimap)
  (CallFunction|ReorderMinimapStack))

(event Custom|PopMinimapFromStack
  (params (Minimap :type BP%20Minimap%20Object%20Reference))
  ;[1 1 1] Adds and removes minimaps from the stack
  (Utilities|Array|RemoveItem (Variables|DO_NOT_EDIT|GetINTERNAL_MinimapStack) Minimap))

(event EventBeginPlay
  (Utilities|FlowControl|Sequence
    (:then_0
      ;[1 1 1] On start, store a copy of the minimap widget if it exists.
      ; OR create one and add it to the viewport if it does not.
      (bind _foundwidgets (Widget|GetAllWidgetsOfClass "/Game/DynamicMinimapSystem/Blueprints/Widgets/Widget_Minimap.Widget_Minimap_C" false))
      (if (> (Utilities|Array|Length _foundwidgets) 0)
        (Variables|DO_NOT_EDIT|SetINTERNAL_MinimapWidget (Utilities|Array|Get(acopy) _foundwidgets))
        (else
          (bind _returnvalue (UserInterface|CreateWidget "/Game/DynamicMinimapSystem/Blueprints/Widgets/Widget_Minimap.Widget_Minimap_C"))
          (bind _output_get (Variables|DO_NOT_EDIT|SetINTERNAL_MinimapWidget _returnvalue))
          (UserInterface|Viewport|AddtoViewport _output_get 0))))
    (:then_1
      ;[1 1 1] Keep checking if everything required is initialised.
      ; Clear timer when initialisation successful.
      (bind _returnvalue_2 (Utilities|Time|SetTimerbyEvent (delegate Custom|AttemptToInitialise) 0.05 true))
      (Variables|DO_NOT_EDIT|SetINTERNAL_CheckMinimapValidTimer _returnvalue_2))))

(fn ConstructionScript
  (bind _areasize (Variables|Default|GetAreaSize))
  (bind _areasize_2 (Variables|Default|GetAreaSize))
  (bind _debugvolume (Variables|Default|GetDebugVolume))
  (bind _returnvalue (* _areasize_2 0.5))
  ;[1 1 1] Update main volume trigger size
  (Components|Box|SetBoxExtent (Variables|Default|GetMinimapVolume_Trigger) (Math|Vector|MakeVector _returnvalue _returnvalue (* (Variables|Default|GetAreaHeight) 0.5)) true)
  ;[1 1 1] Update helper visuals, such as a cube that covers the volume trigger to make it easier to see and select.
  (Transformation|SetWorldScale3D (Variables|Default|GetDebugVolume) (/ (Math|Vector|MakeVector _areasize _areasize (Variables|Default|GetAreaHeight)) 1e+02))
  (if (> (Utilities|Array|Length (Variables|Default|GetCustomAreas)) 0)
    (Rendering|SetVisibility _debugvolume false true)
    (else
      (Rendering|SetVisibility _debugvolume true true))))

(fn IsActorInsideMinimapArea
  (params (Actor :type Actor%20Object%20Reference))
  ;[1 1 1] Checks an actor is inside the minimap volume.
  ; The method to determine this is different depending on if this minimap uses Custom Areas or not.
  (if (Variables|DO_NOT_EDIT|GetINTERNAL_UsesCustomAreas)
    (for _array_element (Variables|Default|GetCustomAreas)
      (if (Default|IsActorInsideRegion _array_element Actor)
        (return true)))
    (return false)
    (else
      (return (Utilities|Array|ContainsItem (Collision|GetOverlappingActors (Variables|Default|GetMinimapVolume_Trigger) "/Game/DynamicMinimapSystem/Blueprints/BP_MinimapDetectorAttachmentObject.BP_MinimapDetectorAttachmentObject_C" :!class /Script/Engine.PrimitiveComponent) Actor)))))

(fn UpdateMinimapBoundsTrigger
  (params (Enabled :type Boolean))
  ;[1 1 1] Update the size and shape of the minimap bounds trigger based on the new minimap settings
  (Default|SetTriggerShape (Variables|DO_NOT_EDIT|GetINTERNAL_MinimapBoundsTrigger) (Variables|Default|GetMinimapShape) (* (/ (Variables|Default|GetAreaSize) 2.0) (Variables|Default|GetZoomOut)) (Variables|Default|GetAreaHeight) Enabled))

(fn UpdateCustomAreas
  (params (Entered :type Boolean))
  ;[1 1 1] Called by the "BP_MinimapCustomArea" blueprint whenever the player enters or leaves a Custom Area associated with this blueprint.
  ; If upon entering, the number of Custom Areas active is 1, then the player has just entered this minimap.
  ; If upon leaving, the number of Custom Areas active is 0, then the player has just exited this minimap.
  (if Entered
    (Math|Integer|IncrementInt (Variables|DO_NOT_EDIT|GetINTERNAL_NumCustomAreasActive)
      (:%20%20
        (if (== (Variables|DO_NOT_EDIT|GetINTERNAL_NumCustomAreasActive) 1)
          (CallFunction|AttemptEnableMinimap))))
    (else
      (Math|Integer|DecrementInt (Variables|DO_NOT_EDIT|GetINTERNAL_NumCustomAreasActive)
        (:%20%20
          (if (== (Variables|DO_NOT_EDIT|GetINTERNAL_NumCustomAreasActive) 0)
            (CallFunction|DisableMinimap true true)))))))

(fn AreAllCustomAreasValid
  ;[1 1 1] This checks to see if all Custom Area blueprints associated with this minimap are loaded and valid.
  (for _array_element (Variables|Default|GetCustomAreas)
    (Utilities|IsValid _array_element
      (:Is%20Not%20Valid
        (return false))))
  (return true))

(fn ShouldOverrideCurrentMinimap
  ;[1 1 1] This checks that the minimap we want to enable has the highest sort order of all minimap volumes the player is currently inside.
  (bind _array_element (Utilities|Array|ForEachLoopwithBreak (Variables|DO_NOT_EDIT|GetINTERNAL_MinimapStack))
    (:LoopBody
      (if (!= _array_element self)
        (if (> (Variables|BP_Minimap_C|GetSortOrder _array_element) (Variables|Default|GetSortOrder))
          (return false))))
    (:Completed
      (return true))))

(fn ReorderMinimapStack
  (bind _internal_minimapstack (Variables|DO_NOT_EDIT|GetINTERNAL_MinimapStack))
  ;[1 1 1] Reorders active minimaps by sort order, so we know which one to re-activate when we leave the current minimap volume.
  (for (_array_element _array_index) _internal_minimapstack
    (for _index (range _array_index (- (Utilities|Array|Length _internal_minimapstack) 1))
      (if (< (Variables|BP_Minimap_C|GetSortOrder (Utilities|Array|Get(acopy) (Variables|DO_NOT_EDIT|GetINTERNAL_MinimapStack) _index)) (Variables|BP_Minimap_C|GetSortOrder _array_element))
        (Utilities|Array|Swap (Variables|DO_NOT_EDIT|GetINTERNAL_MinimapStack) _array_index _index)))))

(fn GetAllOverlappingActors
  ;[1 1 1] Returns all valid minimap actors currently inside the minimap volume.
  ; The method depends on if this minimap uses Custom Areas or not.
  (if (Variables|DO_NOT_EDIT|GetINTERNAL_UsesCustomAreas)
    (Utilities|FlowControl|Sequence
      (:then_0
        (for _array_element (Variables|Default|GetCustomAreas)
          (for _array_element_2 (Default|GetAllOverlappingActors _array_element)
            (Utilities|Array|AddUnique (LocalVariables|GetOverlappedActors) _array_element_2))))
      (:then_1
        (return (LocalVariables|GetOverlappedActors))))
    (else
      (return (Collision|GetOverlappingActors (Variables|Default|GetMinimapVolume_Trigger) "/Game/DynamicMinimapSystem/Blueprints/BP_MinimapDetectorAttachmentObject.BP_MinimapDetectorAttachmentObject_C" :!class /Script/Engine.PrimitiveComponent)))))

(fn CheckHasJustExitedCustomArea
  (params (Actor :type Actor%20Object%20Reference))
  ;[1 1 1] On an actor exiting any Custom Area, check if that actor is still inside any other associated Custom Area.
  ; If not, then they have exited all Custom Areas, and by proxy, this minimap volume.
  (if (Variables|DO_NOT_EDIT|GetINTERNAL_CurrentlyActive)
    (for _array_element (Variables|Default|GetCustomAreas)
      (for _array_element_2 (Variables|/Game/DynamicMinimapSystem/Blueprints/BP_MinimapCustomArea.BP_MinimapCustomArea_C|GetINTERNAL_ActorsEntered _array_element)
        (if (== _array_element_2 Actor)
          (return))))
    (Default|RemoveActortoShow (Variables|DO_NOT_EDIT|GetINTERNAL_MinimapWidget) (Actor|GetComponentbyClass (Actor|GetAttachParentActor Actor) "/Game/DynamicMinimapSystem/Blueprints/Component_MinimapIcon.Component_MinimapIcon_C"))))

(fn CheckActorJustEnteredCustomArea
  (params (Actor :type Actor%20Object%20Reference))
  ;[1 1 1] On an actor entering a Custom Area, check if that actor is already inside any other Custom Area linked to this minimap.
  ; If not, that means the actor has just entered this minimap's Custom Area.
  ; If so, that means they were already within this minimap's bounds, and so have NOT just entered.
  (LocalVariables|SetIncomingActor Actor)
  (if (Variables|DO_NOT_EDIT|GetINTERNAL_CurrentlyActive)
    (bind _array_element (Utilities|Array|ForEachLoopwithBreak (Variables|Default|GetCustomAreas) :!label _label)
      (:LoopBody
        (bind _array_element_2 (Utilities|Array|ForEachLoopwithBreak (Variables|/Game/DynamicMinimapSystem/Blueprints/BP_MinimapCustomArea.BP_MinimapCustomArea_C|GetINTERNAL_ActorsEntered _array_element) :!label _label_2)
          (:LoopBody
            (if (== _array_element_2 (LocalVariables|GetIncomingActor))
              (bind _result (Math|Integer|IncrementInt (LocalVariables|GetNumEntries))
                (:%20%20
                  (if (> _result 1)
                    (LocalVariables|SetOneOverlappingRegionOnly false)
                    (goto _label_2 Break))))))
          (:Completed
            (if (not (LocalVariables|GetOneOverlappingRegionOnly))
              (goto _label Break)))))
      (:Completed
        (if (LocalVariables|GetOneOverlappingRegionOnly)
          (if (Variables|DO_NOT_EDIT|GetINTERNAL_CurrentlyActive)
            (if (Default|IsOverlapping (Variables|DO_NOT_EDIT|GetINTERNAL_MinimapBoundsTrigger) (LocalVariables|GetIncomingActor))
              (Default|AddActortoShow (Variables|DO_NOT_EDIT|GetINTERNAL_MinimapWidget) (Actor|GetComponentbyClass (Actor|GetAttachParentActor (LocalVariables|GetIncomingActor)) "/Game/DynamicMinimapSystem/Blueprints/Component_MinimapIcon.Component_MinimapIcon_C")))))))))

(fn AttemptEnableMinimap
  ;[1 1 1] Push this minimap onto the stack of all active minimaps, so they know which volumes the player is standing in.
  (if (not (Variables|DO_NOT_EDIT|GetINTERNAL_CurrentlyActive))
    (bind _outactors (Actor|GetAllActorsOfClass "BP_Minimap_C"))
    (for _array_element _outactors
      (CallFunction|PushMinimaptoStack _array_element self))
    (if (CallFunction|ShouldOverrideCurrentMinimap)
      ;[1 1 1] Set current minimap active
      (Utilities|FlowControl|Sequence
        (:then_0
          (Variables|DO_NOT_EDIT|SetINTERNAL_CurrentlyActive true)
          (CallFunction|SetWorldCenterObject)
          (CallFunction|StoreMinimapAreaTriggerifNotAlreadySet))
        (:then_1
          (Utilities|FlowControl|Sequence
            (:then_0
              ;[1 1 1] Disable all other active minimaps
              (bind _outactors_2 (Actor|GetAllActorsOfClass "BP_Minimap_C"))
              (for _array_element_2 _outactors_2
                (if (not (== _array_element_2 self))
                  (if (Variables|BP_Minimap_C|GetINTERNAL_CurrentlyActive _array_element_2)
                    (CallFunction|DisableMinimap _array_element_2 false false)))))
            (:then_1
              ;[1 1 1] Initialise the minimap, and display any objects that are within the minimap
              ; volume that are always tracked off screen
              (Default|SetArea (Variables|DO_NOT_EDIT|GetINTERNAL_MinimapWidget) (Variables|Default|GetMinimapImage) (Variables|Default|GetAreaSize) (Variables|Default|GetZoomOut) (Variables|Default|GetShowAreaName) (Variables|Default|GetAreaName) (Variables|Default|GetRotationType) (Variables|Default|GetMinimapShape) self (Variables|Default|GetBorderColour) (Variables|Default|GetTextColour) (Variables|Default|GetTextBackgroundColour) (Variables|Default|GetMinimapScale))
              (CallFunction|UpdateOffscreenTrackedObjects))
            (:then_2
              ;[1 1 1] Update the visibility sphere and minimap widget
              (Transformation|AttachActorToActor (Variables|DO_NOT_EDIT|GetINTERNAL_MinimapBoundsTrigger) (Variables|/Game/DynamicMinimapSystem/Blueprints/Widgets/Widget_Minimap.Widget_Minimap_C|GetWorldCenterObject (Variables|DO_NOT_EDIT|GetINTERNAL_MinimapWidget)) "None" "SnapToTarget" "SnapToTarget" "KeepRelative" true)
              (Default|UpdateMinimap (Variables|DO_NOT_EDIT|GetINTERNAL_MinimapWidget)))))))))

(fn DisableMinimap
  (params (EnableFromStack :type Boolean) (RemoveFromStack :type Boolean))
  (bind _internal_minimapstack (Variables|DO_NOT_EDIT|GetINTERNAL_MinimapStack))
  (bind _returnvalue (Utilities|Array|Length _internal_minimapstack))
  ;[1 1 1] Disable Minimap.
  ; - Clear minimap actors from visibility sphere.
  ; - Remove self from the stack of all other minimaps.
  ; - If the player is inside any other minimap volume, attempt to switch to that minimap.
  (if (Variables|DO_NOT_EDIT|GetINTERNAL_CurrentlyActive)
    (Variables|DO_NOT_EDIT|SetINTERNAL_CurrentlyActive false)
    (Utilities|FlowControl|Sequence
      (:then_0
        (Utilities|IsValid (Variables|DO_NOT_EDIT|GetINTERNAL_MinimapBoundsTrigger)
          (:Is%20Valid
            (CallFunction|UpdateMinimapBoundsTrigger false))
          (:Is%20Not%20Valid
            _))
        (CallFunction|ClearActorsfromVisibilitySphere))
      (:then_1
        (if RemoveFromStack
          (bind _outactors (Actor|GetAllActorsOfClass "BP_Minimap_C"))
          (for _array_element _outactors
            (CallFunction|PopMinimapfromStack _array_element self)))
        (if EnableFromStack
          (if (> _returnvalue 0)
            (CallFunction|AttemptEnableMinimap (Utilities|Array|Get(acopy) _internal_minimapstack (- _returnvalue 1)))))))))

(fn SetWorldCenterObject
  ;[1 1 1] If the minimap should scroll with the player, set the player as the minimap origin.
  ; Otherwise, set the minimap object as the origin.
  (if (Variables|Default|GetMoveWithPlayer)
    (Variables|/Game/DynamicMinimapSystem/Blueprints/Widgets/Widget_Minimap.Widget_Minimap_C|SetWorldCenterObject (Variables|DO_NOT_EDIT|GetINTERNAL_MinimapWidget) (Game|GetPlayerCharacter 0))
    (else
      (Variables|/Game/DynamicMinimapSystem/Blueprints/Widgets/Widget_Minimap.Widget_Minimap_C|SetWorldCenterObject (Variables|DO_NOT_EDIT|GetINTERNAL_MinimapWidget) self))))

(fn StoreMinimapAreaTriggerifNotAlreadySet
  ;[1 1 1] The visibility trigger tracks which objects are near enough to show on the minimap.
  ; If it's already set, then don't need to do anything.
  ; If not set and there's already one in the world (created by another minimap), store it.
  ; Otherwise, create a new one, set its bounds and attach it to the target to be tracked (either the player, or the minimap itself if the map is static)
  (Utilities|IsValid (Variables|DO_NOT_EDIT|GetINTERNAL_MinimapBoundsTrigger)
    (:Is%20Not%20Valid
      (bind _outactors (Actor|GetAllActorsOfClass "/Game/DynamicMinimapSystem/Blueprints/BP_MinimapBoundsTrigger.BP_MinimapBoundsTrigger_C"))
      (if (> (Utilities|Array|Length _outactors) 0)
        (Utilities|IsValid (Utilities|Array|Get(acopy) _outactors)
          (:Is%20Valid
            (Variables|DO_NOT_EDIT|SetINTERNAL_MinimapBoundsTrigger (Utilities|Array|Get(acopy) _outactors))))
        (else
          (bind _returnvalue (Game|SpawnActorfromClass "/Game/DynamicMinimapSystem/Blueprints/BP_MinimapBoundsTrigger.BP_MinimapBoundsTrigger_C" (Math|Transform|MakeTransform (Transformation|GetActorLocation (Variables|/Game/DynamicMinimapSystem/Blueprints/Widgets/Widget_Minimap.Widget_Minimap_C|GetWorldCenterObject (Variables|DO_NOT_EDIT|GetINTERNAL_MinimapWidget)))) "Undefined" 0 0))
          (Variables|DO_NOT_EDIT|SetINTERNAL_MinimapBoundsTrigger _returnvalue)
          (CallFunction|UpdateMinimapBoundsTrigger false)
          (Transformation|AttachActorToActor (Variables|DO_NOT_EDIT|GetINTERNAL_MinimapBoundsTrigger) (Variables|/Game/DynamicMinimapSystem/Blueprints/Widgets/Widget_Minimap.Widget_Minimap_C|GetWorldCenterObject (Variables|DO_NOT_EDIT|GetINTERNAL_MinimapWidget)) "None" "SnapToTarget" "SnapToTarget" "KeepRelative" true))))))

(fn ClearActorsfromVisibilitySphere
  (bind _internal_minimapwidget (Variables|DO_NOT_EDIT|GetINTERNAL_MinimapWidget))
  (bind _internal_minimapwidget_2 (Variables|DO_NOT_EDIT|GetINTERNAL_MinimapWidget))
  (bind _trackactorslist (Variables|/Game/DynamicMinimapSystem/Blueprints/Widgets/Widget_Minimap.Widget_Minimap_C|GetTrackActorsList _internal_minimapwidget_2))
  (bind _alwaystrackedactors (Variables|/Game/DynamicMinimapSystem/Blueprints/Widgets/Widget_Minimap.Widget_Minimap_C|GetAlwaysTrackedActors _internal_minimapwidget))
  ;[1 1 1] Clear all actors that are currently in the visibility sphere, and being displayed on the minimap.
  ; This is called when the minimap is switched to another one, so we want to clear any currently shown icons,
  ; and let the new minimap re-populate the list of visible actors.
  (for _array_element _alwaystrackedactors
    (Utilities|IsValid (Default|INTERNALGetAssociatedWidget _array_element)
      (:Is%20Valid
        (Default|Disable (Default|INTERNALGetAssociatedWidget _array_element))
        (Default|SetAssociatedWidget _array_element))))
  (Utilities|Array|Clear _alwaystrackedactors)
  (for _array_element_2 _trackactorslist
    (Utilities|IsValid (Default|INTERNALGetAssociatedWidget _array_element_2)
      (:Is%20Valid
        (Default|Disable (Default|INTERNALGetAssociatedWidget _array_element_2))
        (Default|SetAssociatedWidget _array_element_2))))
  (Utilities|Array|Clear _trackactorslist))

(fn AttemptInitialisation
  ;[1 1 1] Checks if everything required for the minimap to work is is valid and loaded. If not, will check again in 0.05s, until successful.
  ; On initialised, sets up a few internal variables.
  (Utilities|FlowControl|Sequence
    (:then_0
      (Utilities|IsValid (Variables|DO_NOT_EDIT|GetINTERNAL_MinimapWidget)
        (:Is%20Valid
          (if (> (Utilities|Array|Length (Variables|Default|GetCustomAreas)) 0)
            (Variables|DO_NOT_EDIT|SetINTERNAL_UsesCustomAreas true)
            (if (CallFunction|AreAllCustomAreasValid)
              (for _array_element (Variables|Default|GetCustomAreas)
                (Default|Activate _array_element self))
              (return true))
            (else
              (Collision|SetCollisionEnabled (Variables|Default|GetMinimapVolume_Trigger) "QueryOnly")
              (return true))))))
    (:then_1
      (return false))))

(fn SetZoomOut
  (params (ZoomOut :type Float%20%28single-precision%29))
  ;[1 1 1] Update new zoom out value
  (Utilities|IsValid (Variables|DO_NOT_EDIT|GetINTERNAL_MinimapWidget)
    (:Is%20Valid
      (bind _output_get (Variables|Default|SetZoomOut ZoomOut))
      (Variables|/Game/DynamicMinimapSystem/Blueprints/Widgets/Widget_Minimap.Widget_Minimap_C|SetZoom (Variables|DO_NOT_EDIT|GetINTERNAL_MinimapWidget) _output_get)
      (CallFunction|UpdateOffscreenTrackedObjects))))

(fn UpdateOffscreenTrackedObjects
  ;[1 1 1] Update offscreen tracked objects
  (for _array_element (CallFunction|GetAllOverlappingActors)
    (bind _asbp_minimap_detector_attachment_object (Utilities|Casting|CastToBP_MinimapDetectorAttachmentObject _array_element))
    (Utilities|IsValid (Actor|GetComponentbyClass (Variables|/Game/DynamicMinimapSystem/Blueprints/BP_MinimapDetectorAttachmentObject.BP_MinimapDetectorAttachmentObject_C|GetParentActor _asbp_minimap_detector_attachment_object) "/Game/DynamicMinimapSystem/Blueprints/Component_MinimapIcon.Component_MinimapIcon_C")
      (:Is%20Valid
        (if (Utilities|Enum|NotEqual(Enum) (.OffScreenLogic (Utilities|Struct|BreakSTRUCT_OffscreenRingProperties (Variables|/Game/DynamicMinimapSystem/Blueprints/Component_MinimapIcon.Component_MinimapIcon_C|GetOffScreenLogic (Actor|GetComponentbyClass (Variables|/Game/DynamicMinimapSystem/Blueprints/BP_MinimapDetectorAttachmentObject.BP_MinimapDetectorAttachmentObject_C|GetParentActor _asbp_minimap_detector_attachment_object) "/Game/DynamicMinimapSystem/Blueprints/Component_MinimapIcon.Component_MinimapIcon_C")))) "NewEnumerator0")
          (Default|AddAlwaysTrackedActor (Variables|DO_NOT_EDIT|GetINTERNAL_MinimapWidget) (Actor|GetComponentbyClass (Variables|/Game/DynamicMinimapSystem/Blueprints/BP_MinimapDetectorAttachmentObject.BP_MinimapDetectorAttachmentObject_C|GetParentActor _asbp_minimap_detector_attachment_object) "/Game/DynamicMinimapSystem/Blueprints/Component_MinimapIcon.Component_MinimapIcon_C"))))))
  (CallFunction|UpdateMinimapBoundsTrigger true))

(fn SetAreaName
  (params (AreaName :type Text))
  ;[1 1 1] Update area name
  (Utilities|IsValid (Variables|DO_NOT_EDIT|GetINTERNAL_MinimapWidget)
    (:Is%20Valid
      (bind _output_get (Variables|Default|SetAreaName AreaName))
      (Rendering|Components|TextRender|SetText (Variables|/Game/DynamicMinimapSystem/Blueprints/Widgets/Widget_Minimap.Widget_Minimap_C|GetAreaNameText (Variables|DO_NOT_EDIT|GetINTERNAL_MinimapWidget)) _output_get))))

(fn SetAreaNameColour
  (params (Colour :type Linear%20Color%20Structure))
  ;[1 1 1] Update area name colour
  (Utilities|IsValid (Variables|DO_NOT_EDIT|GetINTERNAL_MinimapWidget)
    (:Is%20Valid
      (bind _output_get (Variables|Default|SetTextColour Colour))
      (Appearance|SetColorandOpacity (Variables|/Game/DynamicMinimapSystem/Blueprints/Widgets/Widget_Minimap.Widget_Minimap_C|GetAreaNameText (Variables|DO_NOT_EDIT|GetINTERNAL_MinimapWidget)) (Utilities|Struct|MakeSlateColor _output_get) :!class /Script/UMG.TextBlock))))