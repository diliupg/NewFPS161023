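; Actor component that gives its owner a minimap icon and an optional in-world icon.
; On BeginPlay it spawns a detector attachment object, which drives the in-world icon and serves minimap bounds checks.
; Off-screen-tracked icons tick until the minimap initialises, then register as always tracked if inside its area.
; Setters update the in-world icon or assigned minimap widget, while SetState shows, hides or permanently destroys the icons.
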(event Custom|SetAssociatedWidget
  (params (Widget :type Widget%20Minimap%20Icon%20Object%20Reference))
  ;[1 1 1] Sets the available Widget that will be used to show this minimap icon
  (Variables|D_NOT_EDIT|SetINTERNAL_AssociatedWidget Widget)
  (Utilities|IsValid Widget
    (:Is%20Valid
      (Variables|/Game/DynamicMinimapSystem/Blueprints/Widgets/Widget_MinimapIcon.Widget_MinimapIcon_C|SetShouldRotate Widget (Variables|IconMinimap|GetRotatesWithActor)))))

(event EventBeginPlay
  ;[1 1 1] On Begin Play, spawn a Minimap Attachment object, and attach it to the parent actor. This object is checked by the minimap trigger to see if it's inside its bounds.
  ; Initialise the icon, such as size, colour, animation type...etc.
  ; If it is set to be tracked off screen, enable tick and wait for the Minimap to become valid (then add self to its list of "always tracked" actors).
  (bind _returnvalue (Game|SpawnActorfromClass "/Game/DynamicMinimapSystem/Blueprints/BP_MinimapDetectorAttachmentObject.BP_MinimapDetectorAttachmentObject_C" (Math|Transform|MakeTransform (Transformation|GetActorLocation (Components|GetOwner))) "Undefined" 0 0))
  (bind _output_get (Variables|D_NOT_EDIT|SetINTERNAL_MinimapAttachmentObject _returnvalue))
  (Default|SetActive _output_get (Variables|General|GetIconsEnabled))
  (Default|Initialise _output_get (Components|GetOwner) (Variables|IconWorld|GetShowIconInWorld) (Variables|IconWorld|GetInWorldIcon) (Variables|IconWorld|GetInWorldIconZOffset) (Variables|IconWorld|GetInWorldIconTint) (Variables|IconWorld|GetInWorldIconScale) (Variables|IconWorld|GetInWorldAnimationType))
  (if (Utilities|Enum|Equal(Enum) (.OffScreenLogic (Utilities|Struct|BreakSTRUCT_OffscreenRingProperties (Variables|IconMinimap|GetOffScreenLogic))) "NewEnumerator1")
    (Components|Tick|SetComponentTickEnabled true)))

(event EventTick
  (params (DeltaSeconds :type Float%20%28single-precision%29))
  ;[1 1 1] If this icon is set to be tracked off screen, keep checking each tick until the minimap is loaded and valid.
  ; Then check if this actor is inside the minimap region. If so, add this icon to the minimap to be tracked offscreen.
  (bind _foundwidgets (Widget|GetAllWidgetsOfClass "/Game/DynamicMinimapSystem/Blueprints/Widgets/Widget_Minimap.Widget_Minimap_C" true))
  (if (> (Utilities|Array|Length _foundwidgets) 0)
    (Utilities|IsValid (Utilities|Array|Get(acopy) _foundwidgets)
      (:Is%20Valid
        (Utilities|IsValid (Variables|/Game/DynamicMinimapSystem/Blueprints/Widgets/Widget_Minimap.Widget_Minimap_C|GetMinimapObject (Utilities|Array|Get(acopy) _foundwidgets))
          (:Is%20Valid
            (if (Variables|/Game/DynamicMinimapSystem/Blueprints/BP_Minimap.BP_Minimap_C|GetINTERNAL_IsInitialised (Variables|/Game/DynamicMinimapSystem/Blueprints/Widgets/Widget_Minimap.Widget_Minimap_C|GetMinimapObject (Utilities|Array|Get(acopy) _foundwidgets)))
              (Components|Tick|SetComponentTickEnabled false)
              (if (Default|IsActorInsideMinimapArea (Variables|/Game/DynamicMinimapSystem/Blueprints/Widgets/Widget_Minimap.Widget_Minimap_C|GetMinimapObject (Utilities|Array|Get(acopy) _foundwidgets)) (Variables|D_NOT_EDIT|GetINTERNAL_MinimapAttachmentObject))
                (Default|AddAlwaysTrackedActor (Utilities|Array|Get(acopy) _foundwidgets) self)))))))))

(fn INTERNALGetAssociatedWidget
  ;[1 1 1] Returns the widget that will display this icon on the minimap. This WILL be
  ; null if the parent actor is not within the minimap region, and not set to be
  ; tracked off screen. This is normal, it will be NULL often.
  (return (Variables|D_NOT_EDIT|GetINTERNAL_AssociatedWidget)))

(fn SetinWorldImage
  (params (Image :type Texture%202D%20Object%20Reference))
  ;[1 1 1] Set the in-world icon to be displayed, read from the associated Minimap Attachment Object.
  (Utilities|IsValid (Variables|D_NOT_EDIT|GetINTERNAL_MinimapAttachmentObject)
    (:Is%20Valid
      (Default|SetImage (Default|GetinWorldWidget (Variables|D_NOT_EDIT|GetINTERNAL_MinimapAttachmentObject)) Image))))

(fn SetinWorldScale
  (params (Scale :type Float%20%28single-precision%29))
  ;[1 1 1] Set the scale of the in-world icon, read from the associated Minimap Attachment Object.
  (Utilities|IsValid (Variables|D_NOT_EDIT|GetINTERNAL_MinimapAttachmentObject)
    (:Is%20Valid
      (Default|SetScale (Default|GetinWorldWidget (Variables|D_NOT_EDIT|GetINTERNAL_MinimapAttachmentObject)) Scale))))

(fn SetinWorldTint
  (params (Tint :type Linear%20Color%20Structure :default "(R=1.000000,G=1.000000,B=1.000000,A=1.000000)"))
  ;[1 1 1] Set the tint of the in-world icon, read from the associated Minimap Attachment Object.
  (Utilities|IsValid (Variables|D_NOT_EDIT|GetINTERNAL_MinimapAttachmentObject)
    (:Is%20Valid
      (Default|SetTint (Default|GetinWorldWidget (Variables|D_NOT_EDIT|GetINTERNAL_MinimapAttachmentObject)) Tint))))

(fn SetinWorldAnimationType
  (params (AnimationType :type ENUM_MinimapIconAnimationType%20Enum :default "NewEnumerator3"))
  ;[1 1 1] Set the animation type of the in-world icon, read from the associated Minimap Attachment Object.
  (Utilities|IsValid (Variables|D_NOT_EDIT|GetINTERNAL_MinimapAttachmentObject)
    (:Is%20Valid
      (Default|SetAnimationType (Default|GetinWorldWidget (Variables|D_NOT_EDIT|GetINTERNAL_MinimapAttachmentObject)) AnimationType))))

(fn SetinWorldZOffset
  (params (OffsetZ :type Float%20%28single-precision%29))
  ;[1 1 1] Set the Z-offset of the in-world icon, read from the associated Minimap Attachment Object.
  (Utilities|IsValid (Variables|D_NOT_EDIT|GetINTERNAL_MinimapAttachmentObject)
    (:Is%20Valid
      (Default|SetZOffset (Variables|D_NOT_EDIT|GetINTERNAL_MinimapAttachmentObject) OffsetZ))))

(fn SetMinimapImage
  (params (Image :type Texture%202D%20Object%20Reference))
  ;[1 1 1] Set the minimap icon to be displayed, read from the associated Minimap Attachment Object.
  (bind _output_get (Variables|IconMinimap|SetMinimapIcon Image))
  (Utilities|IsValid (Variables|D_NOT_EDIT|GetINTERNAL_AssociatedWidget)
    (:Is%20Valid
      (Default|SetImage (Variables|D_NOT_EDIT|GetINTERNAL_AssociatedWidget) _output_get))))

(fn SetMinimapScale
  (params (Scale :type Float%20%28single-precision%29))
  ;[1 1 1] Set the minimap icon scale, read from the associated Minimap Attachment Object.
  (bind _output_get (Variables|IconMinimap|SetMinimapIconScale Scale))
  (Utilities|IsValid (Variables|D_NOT_EDIT|GetINTERNAL_AssociatedWidget)
    (:Is%20Valid
      (Default|SetScale (Variables|D_NOT_EDIT|GetINTERNAL_AssociatedWidget) _output_get))))

(fn SetMinimapTint
  (params (Colour :type Linear%20Color%20Structure :default "(R=1.000000,G=1.000000,B=1.000000,A=1.000000)"))
  ;[1 1 1] Set the minimap icon tint, read from the associated Minimap Attachment Object.
  (bind _output_get (Variables|IconMinimap|SetMinimapTint Colour))
  (Utilities|IsValid (Variables|D_NOT_EDIT|GetINTERNAL_AssociatedWidget)
    (:Is%20Valid
      (Default|SetTint (Variables|D_NOT_EDIT|GetINTERNAL_AssociatedWidget) _output_get))))

(fn SetMinimapAnimationType
  (params (AnimationType :type ENUM_MinimapIconAnimationType%20Enum :default "NewEnumerator3"))
  ;[1 1 1] Set the minimap icon animation type, read from the associated Minimap Attachment Object.
  (bind _output_get (Variables|IconMinimap|SetMinimapAnimationType AnimationType))
  (Utilities|IsValid (Variables|D_NOT_EDIT|GetINTERNAL_AssociatedWidget)
    (:Is%20Valid
      (Default|SetAnimationType (Variables|D_NOT_EDIT|GetINTERNAL_AssociatedWidget) _output_get))))

(fn SetState
  (params (MinimapState :type ENUM_MinimapIconState%20Enum :default "NewEnumerator0"))
  (bind _self self)
  (bind _internal_minimapattachmentobject (Variables|D_NOT_EDIT|GetINTERNAL_MinimapAttachmentObject))
  ;[1 1 1] Sets the component to be shown, temporarily hidden, or should be destroyed forever (for example if a quest NPC no longer needs its quest icons)
  (switch Utilities|FlowControl|Switch|SwitchonENUM_MinimapIconState MinimapState
    (:NewEnumerator0
      (Variables|General|SetIconsEnabled true)
      (Default|SetActive (Variables|D_NOT_EDIT|GetINTERNAL_MinimapAttachmentObject) true)
      (if (Utilities|Enum|Equal(Enum) (.OffScreenLogic (Utilities|Struct|BreakSTRUCT_OffscreenRingProperties (Variables|IconMinimap|GetOffScreenLogic))) "NewEnumerator1")
        (bind _foundwidgets (Widget|GetAllWidgetsOfClass "/Game/DynamicMinimapSystem/Blueprints/Widgets/Widget_Minimap.Widget_Minimap_C" true))
        (if (> (Utilities|Array|Length _foundwidgets) 0)
          (Utilities|IsValid (Utilities|Array|Get(acopy) _foundwidgets)
            (:Is%20Valid
              (Default|AddAlwaysTrackedActor (Utilities|Array|Get(acopy) _foundwidgets) self))))))
    (:NewEnumerator1
      (Variables|General|SetIconsEnabled false :!label _label)
      (Utilities|FlowControl|Sequence
        (:then_0
          (bind _foundwidgets_2 (Widget|GetAllWidgetsOfClass "/Game/DynamicMinimapSystem/Blueprints/Widgets/Widget_Minimap.Widget_Minimap_C" true))
          (if (> (Utilities|Array|Length _foundwidgets_2) 0)
            (Utilities|IsValid (Utilities|Array|Get(acopy) _foundwidgets_2)
              (:Is%20Valid
                (Utilities|FlowControl|Sequence
                  (:then_0
                    (if (Utilities|Enum|Equal(Enum) (.OffScreenLogic (Utilities|Struct|BreakSTRUCT_OffscreenRingProperties (Variables|IconMinimap|GetOffScreenLogic))) "NewEnumerator1")
                      (Default|RemoveAlwaysTrackedActor (Utilities|Array|Get(acopy) _foundwidgets_2) _self)))
                  (:then_1
                    (Default|RemoveActortoShow (Utilities|Array|Get(acopy) _foundwidgets_2) _self)))))))
        (:then_1
          (Default|SetActive _internal_minimapattachmentobject false)
          (Development|SetHiddeninGame (Variables|/Game/DynamicMinimapSystem/Blueprints/BP_MinimapDetectorAttachmentObject.BP_MinimapDetectorAttachmentObject_C|GetWidget_InWorldIcon _internal_minimapattachmentobject) true true))))
    (:NewEnumerator2
      (Utilities|FlowControl|Sequence
        (:then_0
          (goto _label))
        (:then_1
          (Actor|DestroyActor (Variables|D_NOT_EDIT|GetINTERNAL_MinimapAttachmentObject)))))))