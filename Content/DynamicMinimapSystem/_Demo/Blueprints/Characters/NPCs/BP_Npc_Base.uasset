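; Base NPC for the minimap system demo that walks a looping path through an array of waypoint actors.
; BeginPlay sends it to the first waypoint, if any exist, using AI MoveTo.
; PrepareNextWaypoint advances the index, wrapping to zero after the last entry, then starts the next move.
; Move completion is not handled here, so advancing relies on an external call to PrepareNextWaypoint.
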(event Custom|MoveToNextWaypoint
  ;[1 1 1] Set the NPC to move towards the next waypoint
  (AI|AIMoveTo self "0, 0, 0" (Variables|Default|GetNextWaypoint) 5.0 false))

(event EventBeginPlay
  ;[1 1 1] If NPC has waypoints, start moving them towards the first one in the array.
  (if (> (Utilities|Array|Length (Variables|Default|GetWaypoints)) 0)
    (Variables|Default|SetNextWaypoint (Utilities|Array|Get(acopy) (Variables|Default|GetWaypoints)))
    (CallFunction|MovetoNextWaypoint)))

(fn ConstructionScript)

(fn GetNextWaypoint
  ;[1 1 1] Gets the next waypoint in the array
  (return (Utilities|Array|Get(acopy) (Variables|Default|GetWaypoints) (Variables|Default|GetNextWaypointIndex))))

(fn PrepareNextWaypoint
  ;[1 1 1] Works out what the next waypoint should be.
  ; Is either the next waypoint in the array, OR the first waypoint if the current waypoint is the last one in the array (allowing looped pathing)
  ; Then tells the NPC to move to that waypoint.
  (if (== (- (Utilities|Array|Length (Variables|Default|GetWaypoints)) 1) (Variables|Default|GetNextWaypointIndex))
    (Variables|Default|SetNextWaypointIndex 0)
    (else
      (Math|Integer|IncrementInt (Variables|Default|GetNextWaypointIndex)
        (:%20%20
          _))))
  (Variables|Default|SetNextWaypoint (Utilities|Array|Get(acopy) (Variables|Default|GetWaypoints) (Variables|Default|GetNextWaypointIndex)))
  (CallFunction|MovetoNextWaypoint))